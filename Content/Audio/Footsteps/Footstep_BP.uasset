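; Footstep animation notify that plays a surface-dependent step sound under the mesh's owning actor.
; On notify it line traces 100 units down from the owner's location on the Visibility channel, ignoring the owner.
; The hit's surface type selects a wood step sound or the default concrete cue.
; The sound plays at the impact location through the Multiplayer server call, with the owner passed as sender.
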(fn ReceivedNotify
  (params (MeshComp :type Skeletal%20Mesh%20Component%20Object%20Reference) (Animation :type Anim%20Sequence%20Base%20Object%20Reference) (EventReference :type Anim%20Notify%20Event%20Reference%20Structure%20%28by%20ref%29))
  (bind _returnvalue (Components|GetOwner MeshComp))
  (bind _returnvalue_2 (Transformation|GetActorLocation _returnvalue))
  (bind (_x _y _z) (Math|Vector|BreakVector _returnvalue_2))
  (bind (_outhit _returnvalue_3) (Collision|LineTraceByChannel _returnvalue_2 (Math|Vector|MakeVector _x _y (- _z 1e+02)) "TraceTypeQuery1" false (Utilities|Array|MakeArray _returnvalue) "None"))
  (if _returnvalue_3
    (Default|PlaySoundatLocationServer (Variables|Default|GetMultiplayer) (Utilities|Select :Index (Collision|GetSurfaceType _outhit) :SurfaceType_Default "/Game/Audio/Footsteps/Concrete/Concrete_Step_Cue.Concrete_Step_Cue" :SurfaceType1 "/Game/Audio/Footsteps/Wood/Step_Wood.Step_Wood") (.Location (Collision|BreakHitResult _outhit)) _returnvalue)
    (return false)
    (else
      (return false))))