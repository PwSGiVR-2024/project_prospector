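; Actor that shows floating damage text in the world through a widget component.
; On BeginPlay it creates a W_FloatingText widget from its damage text and critical flag, then sets a short lifespan, longer for critical hits.
; Each Tick it nudges the widget upward by a random amount, with a different range for critical hits.
; The rise is applied per frame without delta time, so its speed depends on frame rate.
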(event EventBeginPlay
  (bind _iscritical (Variables|Default|GetIsCritical))
  ;[1 1 1] Adding widget to this actor
  (bind _returnvalue (UserInterface|CreateWidget "/Game/WeaponComponent/UMG/W_FloatingText.W_FloatingText_C" 0 (Variables|Default|GetDamageText) _iscritical))
  (UserInterface|SetWidget (Variables|Default|GetTextWidget) _returnvalue)
  ;[1 1 1] Destroy actor after 1 sec or 1.5 sec if was critical damage
  (Actor|SetLifeSpan (Math|Float|SelectFloat 1.5 1.0 _iscritical)))

(event EventTick
  (params (DeltaSeconds :type Float%20%28single-precision%29))
  (bind _textwidget (Variables|Default|GetTextWidget))
  ;[1 1 1] Moving Text Up
  (Transformation|SetRelativeLocation _textwidget (+ (Variables|/Script/Engine.SceneComponent|GetRelativeLocation _textwidget) (Math|Vector|MakeVector 0.0 0.0 (Math|Random|RandomFloatinRange 0.5 (Math|Float|SelectFloat 0.25 2.0 (Variables|Default|GetIsCritical))))) false false))

(fn ConstructionScript)