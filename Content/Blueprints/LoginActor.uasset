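; LoginActor is an actor that moves a given player to the Prototype_map level through the main menu game mode.
; ServerChangeMapForClient passes the player to the płacz event, which casts the current game mode to MainMenuGameMode and calls ChangeMapForPlayer.
; Debug prints trace each step, and a failed cast prints the current game mode's name.
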(event Custom|ServerChangeMapForClient
  (params (SpecificPlayer :type Player%20Controller%20Object%20Reference))
  (CallFunction|Płacz SpecificPlayer)
  (Development|PrintString "1"))

(event Custom|płacz
  (params (SpecificPlayer :type Player%20Controller%20Object%20Reference))
  (bind _returnvalue (Game|GetGameMode))
  (Development|PrintString "Hello")
  (bind _asmain_menu_game_mode (Utilities|Casting|CastToMainMenuGameMode _returnvalue)
    (:then
      (Default|ChangeMapforPlayer _asmain_menu_game_mode SpecificPlayer "Prototype_map")
      (Development|PrintString "test"))
    (:CastFailed
      (Development|PrintString (Utilities|GetDisplayName _returnvalue)))))

(event EventBeginPlay
  (Development|PrintString "asdasdasdas"))

(fn ConstructionScript)