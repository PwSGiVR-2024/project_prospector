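; Weapon holder component that handles hitscan shooting, impact feedback and hit markers for its owning character.
; ShootFunction traces from the follow camera and scales weapon damage by a distance falloff curve.
; Damage, tag-based impact effects and sounds, and blood decals from a second trace behind flesh hits go through the owner's MultiplayerFunctions component.
; Flesh hits also show a locally created screen-projected hit marker, which Tick moves off-screen after a short timer.
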(event EventTick
  (params (DeltaSeconds :type Float%20%28single-precision%29))
  (bind _hitmarkerwidgetreference (Variables|Default|GetHitMarkerWidgetReference))
  (if (> (Variables|Default|Gethitmarktime) 0.0)
    (Variables|Default|Sethitmarktime (- (Variables|Default|Gethitmarktime) DeltaSeconds))
    (elif (Utilities|IsValid _hitmarkerwidgetreference)
      (Class|UserWidget|SetPositioninViewport _hitmarkerwidgetreference "(X=-100.000000,Y=0.000000)" true))))

(event EventBeginPlay
  (bind _returnvalue (Components|GetOwner))
  (Variables|Default|SetMultiplayerEvents (Actor|GetComponentbyClass _returnvalue "/Game/Blueprints/MultiplayerFunctions.MultiplayerFunctions_C"))
  (if (Pawn|IsLocallyControlled (Variables|/Script/Engine.Actor|GetInstigator _returnvalue))
    (bind _returnvalue_2 (UserInterface|CreateWidget "/Game/Blueprints/Widgets/HitMarkerWidget.HitMarkerWidget_C" (Game|GetPlayerController 0)))
    (bind _output_get (Variables|Default|SetHitMarkerWidgetReference _returnvalue_2))
    (UserInterface|Viewport|AddtoViewport _output_get 0)
    (Class|UserWidget|SetPositioninViewport (Variables|Default|GetHitMarkerWidgetReference) "(X=0.000000,Y=0.000000)" true)))

(fn ShootFunction
  (bind _multiplayerevents (Variables|Default|GetMultiplayerEvents))
  (bind _multiplayerevents_2 (Variables|Default|GetMultiplayerEvents))
  (bind _multiplayerevents_3 (Variables|Default|GetMultiplayerEvents))
  (bind _multiplayerevents_4 (Variables|Default|GetMultiplayerEvents))
  (bind _followcam (Class|IPlayerInterface|IFGetFollowCamera(Message) (Components|GetOwner)))
  (bind (_outhit _returnvalue) (Collision|LineTraceByChannel (Transformation|GetWorldLocation _followcam) (+ (Transformation|GetWorldLocation _followcam) (* (Math|Vector|GetForwardVector _followcam) 1e+06)) "TraceTypeQuery2" false 0 "None"))
  (if _returnvalue
    (bind _output_get (Variables|Default|SetHitLocation (.ImpactPoint (Collision|BreakHitResult _outhit))))
    (bind _output_get_2 (Variables|Default|SetHitActor (.HitActor (Collision|BreakHitResult _outhit))))
    (Variables|Default|SetHitRotation (Math|Conversions|RotationFromXVector (.ImpactNormal (Collision|BreakHitResult _outhit))))
    (bind _damage (CallFunction|CalcualteDamage _output_get))
    (Default|ApplyDamageServer (Variables|Default|GetMultiplayerEvents) _output_get_2 _damage 0 (Components|GetOwner) "/Engine/EngineDamageTypes/DmgTypeBP_Environmental.DmgTypeBP_Environmental_C")
    (for _array_element (Variables|/Script/Engine.Actor|GetTags _output_get_2)
      (switch name _array_element
        (:Default
          ;[1 1 1] Other hit
          (Default|SpawnEmitteratLocationServer _multiplayerevents "/Game/MilitaryWeapSilver/FX/P_Impact_Stone_Small_01.P_Impact_Stone_Small_01" (Variables|Default|GetHitLocation) (Variables|Default|GetHitRotation) "1.000000,1.000000,1.000000")
          (Default|PlaySoundatLocationServer _multiplayerevents (Variables|/Game/DataAssets/Audio/DAC_ImpactSound.DAC_ImpactSound_C|GetOtherHit (Variables|Default|GetImpactSounds)) (Variables|Default|GetHitLocation))
          (return))
        (:Metal
          ;[1 1 1] Metal hit
          (Default|SpawnEmitteratLocationServer _multiplayerevents_2 "/Game/MilitaryWeapSilver/FX/P_Impact_Metal_Small_01.P_Impact_Metal_Small_01" (Variables|Default|GetHitLocation) (Variables|Default|GetHitRotation) "1.000000,1.000000,1.000000")
          (Default|PlaySoundatLocationServer _multiplayerevents_2 (Variables|/Game/DataAssets/Audio/DAC_ImpactSound.DAC_ImpactSound_C|GetMetalHit (Variables|Default|GetImpactSounds)) (Variables|Default|GetHitLocation))
          (return))
        (:Wood
          ;[1 1 1] Wood hit
          (Default|SpawnEmitteratLocationServer _multiplayerevents_3 "/Game/MilitaryWeapSilver/FX/P_Impact_Wood_Medium_01.P_Impact_Wood_Medium_01" (Variables|Default|GetHitLocation) (Variables|Default|GetHitRotation) "1.000000,1.000000,1.000000")
          (Default|PlaySoundatLocationServer _multiplayerevents_3 (Variables|/Game/DataAssets/Audio/DAC_ImpactSound.DAC_ImpactSound_C|GetWoodHit (Variables|Default|GetImpactSounds)) (Variables|Default|GetHitLocation))
          (return))
        (:Flesh
          ;[1 1 1] Flesh hit
          (Default|SpawnSystematLocationServer _multiplayerevents_4 "/Game/Decals/NS_Blood.NS_Blood" (Variables|Default|GetHitLocation) (Variables|Default|GetHitRotation) "1.000000,1.000000,1.000000")
          (Default|PlaySoundatLocationServer _multiplayerevents_4 (Variables|/Game/DataAssets/Audio/DAC_ImpactSound.DAC_ImpactSound_C|GetFleshHit (Variables|Default|GetImpactSounds)) (Variables|Default|GetHitLocation))
          (Audio|PlaySound2D "/Game/Audio/ImpactSounds/hitmarker.hitmarker" 1.0 1.3 0.1 0 0)
          (Class|UserWidget|SetPositioninViewport (Variables|Default|GetHitMarkerWidgetReference) (.ScreenPosition (Class|GameplayStatics|ProjectWorldtoScreen (Game|GetPlayerController 0) (Variables|Default|GetHitLocation) true)) true)
          (Variables|Default|Sethitmarktime 0.2)
          ;[1 1 1] Spawn blood
          (bind _followcam_2 (Class|IPlayerInterface|IFGetFollowCamera(Message) (Components|GetOwner)))
          (bind _outhit_2 (Collision|LineTraceByChannel (Variables|Default|GetHitLocation) (+ (Variables|Default|GetHitLocation) (* (Math|Vector|GetForwardVector _followcam_2) 5e+02)) "TraceTypeQuery1" false (Utilities|Array|MakeArray (Variables|Default|GetHitActor)) "None"))
          (if true
            (Default|SpawnActortoServer (Variables|Default|GetMultiplayerEvents) "/Game/Blueprints/Decals/BP_BloodDecal.BP_BloodDecal_C" (Math|Transform|MakeTransform (.Location (Collision|BreakHitResult _outhit_2)) (Math|Conversions|RotationFromXVector (.Normal (Collision|BreakHitResult _outhit_2)))) "Undefined")
            (return)))))
    (switch name _array_element
      (:Default
        (Default|SpawnEmitteratLocationServer _multiplayerevents "/Game/MilitaryWeapSilver/FX/P_Impact_Stone_Small_01.P_Impact_Stone_Small_01" (Variables|Default|GetHitLocation) (Variables|Default|GetHitRotation) "1.000000,1.000000,1.000000")
        (Default|PlaySoundatLocationServer _multiplayerevents (Variables|/Game/DataAssets/Audio/DAC_ImpactSound.DAC_ImpactSound_C|GetOtherHit (Variables|Default|GetImpactSounds)) (Variables|Default|GetHitLocation))
        (return))
      (:Metal
        (Default|SpawnEmitteratLocationServer _multiplayerevents_2 "/Game/MilitaryWeapSilver/FX/P_Impact_Metal_Small_01.P_Impact_Metal_Small_01" (Variables|Default|GetHitLocation) (Variables|Default|GetHitRotation) "1.000000,1.000000,1.000000")
        (Default|PlaySoundatLocationServer _multiplayerevents_2 (Variables|/Game/DataAssets/Audio/DAC_ImpactSound.DAC_ImpactSound_C|GetMetalHit (Variables|Default|GetImpactSounds)) (Variables|Default|GetHitLocation))
        (return))
      (:Wood
        (Default|SpawnEmitteratLocationServer _multiplayerevents_3 "/Game/MilitaryWeapSilver/FX/P_Impact_Wood_Medium_01.P_Impact_Wood_Medium_01" (Variables|Default|GetHitLocation) (Variables|Default|GetHitRotation) "1.000000,1.000000,1.000000")
        (Default|PlaySoundatLocationServer _multiplayerevents_3 (Variables|/Game/DataAssets/Audio/DAC_ImpactSound.DAC_ImpactSound_C|GetWoodHit (Variables|Default|GetImpactSounds)) (Variables|Default|GetHitLocation))
        (return))
      (:Flesh
        (Default|SpawnSystematLocationServer _multiplayerevents_4 "/Game/Decals/NS_Blood.NS_Blood" (Variables|Default|GetHitLocation) (Variables|Default|GetHitRotation) "1.000000,1.000000,1.000000")
        (Default|PlaySoundatLocationServer _multiplayerevents_4 (Variables|/Game/DataAssets/Audio/DAC_ImpactSound.DAC_ImpactSound_C|GetFleshHit (Variables|Default|GetImpactSounds)) (Variables|Default|GetHitLocation))
        (Audio|PlaySound2D "/Game/Audio/ImpactSounds/hitmarker.hitmarker" 1.0 1.3 0.1 0 0)
        (Class|UserWidget|SetPositioninViewport (Variables|Default|GetHitMarkerWidgetReference) (.ScreenPosition (Class|GameplayStatics|ProjectWorldtoScreen (Game|GetPlayerController 0) (Variables|Default|GetHitLocation) true)) true)
        (Variables|Default|Sethitmarktime 0.2)
        (bind _followcam_3 (Class|IPlayerInterface|IFGetFollowCamera(Message) (Components|GetOwner)))
        (bind _outhit_3 (Collision|LineTraceByChannel (Variables|Default|GetHitLocation) (+ (Variables|Default|GetHitLocation) (* (Math|Vector|GetForwardVector _followcam_3) 5e+02)) "TraceTypeQuery1" false (Utilities|Array|MakeArray (Variables|Default|GetHitActor)) "None"))
        (if true
          (Default|SpawnActortoServer (Variables|Default|GetMultiplayerEvents) "/Game/Blueprints/Decals/BP_BloodDecal.BP_BloodDecal_C" (Math|Transform|MakeTransform (.Location (Collision|BreakHitResult _outhit_3)) (Math|Conversions|RotationFromXVector (.Normal (Collision|BreakHitResult _outhit_3)))) "Undefined")
          (return))))
    (else
      (return))))

(fn CalcualteDamage
  (params (HitPoint :type Vector))
  (bind _currentweapon (Variables|Default|GetCurrentWeapon))
  (return (Math|Conversions|ToFloat(Integer) (Math|Float|Floor (* (Math|Curves|GetFloatValue (Variables|/Game/DataAssets/Weapons/DAC_Weapon.DAC_Weapon_C|GetDamageFallof _currentweapon) (Math|Vector|Distance(Vector) HitPoint (.location (Transformation|GetActorTransform (Components|GetOwner))))) (Variables|/Game/DataAssets/Weapons/DAC_Weapon.DAC_Weapon_C|GetDamage _currentweapon))))))