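; MainGameInstance is the game instance that connects the game to the GameJolt API for user login and session tracking.
; InitClient initializes the client with the game ID and private key, and Login authenticates a user, then opens a session.
; An opened session starts a looping 45-second timer that pings it as active, and Shutdown closes it.
; Leftover debug prints and a hardcoded test login are disconnected.
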(event Custom|OpenSession
  ;[1 1 1] GameJolt API
  (bind _error (|OpenSession)
    (:Success
      (CallFunction|StartSessionPinging))))

(event Custom|Login
  (params (username :type String) (userToken :type String))
  ;[1 1 1] GameJolt API
  (|Login username userToken
    (:Success
      (Development|PrintString username)
      (CallFunction|OpenSession))))

(event Custom|StartSessionPinging
  ;[1 1 1] GameJolt API
  (Utilities|Time|SetTimerbyEvent (delegate Custom|PingSession) 45.0 true))

(event Custom|PingSession
  ;[1 1 1] GameJolt API
  (|PingSession "active"))

(event Custom|CloseSession
  ;[1 1 1] GameJolt API
  (|CloseSession))

(event Custom|InitClient
  ;[1 1 1] GameJolt API init
  (Class|GameJolt|Initialize 901771 "ac0341805621615d269bf8a9621e5903"))

(event EventShutdown
  ;[1 1 1] GameJoltAPI Shutdown
  (CallFunction|CloseSession))