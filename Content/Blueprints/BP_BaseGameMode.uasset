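; Base game mode that tracks player identities and can move an individual player to another map.
; RegisterPlayer gives each MainPlayerController an incrementing NetID and stores its name in the Users map, which GetPlayerName reads by ID.
; ChangeMapForPlayer runs a clienttravel console command on the specified player.
; RespawnRequested and PlayerDied are empty events, and both map travel and name lookup print debug strings.
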(event Custom|RespawnRequested
  (params (PlayerController :type Main%20Player%20Controller%20Object%20Reference) (Location :type Transform)))

(event Custom|RegisterPlayer
  (params (Controller :type Controller%20Object%20Reference) (Name :type String%20%28by%20ref%29))
  (bind _asmain_player_controller (Utilities|Casting|CastToMainPlayerController Controller))
  (bind _output_get (Variables|/Game/Blueprints/MainPlayerController.MainPlayerController_C|SetNetID _asmain_player_controller (Variables|Default|GetCurrentBiggestID)))
  (Variables|Default|SetCurrentBiggestID (+ (Variables|Default|GetCurrentBiggestID) 1))
  (Utilities|Map|Add (Variables|Default|GetUsers) _output_get Name))

(event Custom|PlayerDied
  (params (Who%20Died :type BP%20Third%20Person%20Character%20Object%20Reference) (Who%20Killed :type Actor%20Object%20Reference)))

(event Custom|ChangeMapForPlayer
  (params (SpecificPlayer :type Player%20Controller%20Object%20Reference) (Map%20name :type String))
  (bind _returnvalue (Utilities|String|Append "clienttravel " Map%20name))
  (Development|ExecuteConsoleCommand _returnvalue SpecificPlayer)
  (Development|PrintString _returnvalue))

(event EventBeginPlay)

(fn ConstructionScript)

(fn GetPlayerName
  (params (UniqueNetID :type Integer%20%28by%20ref%29))
  (bind _users (Variables|Default|GetUsers))
  (bind _value (Utilities|Map|Find _users UniqueNetID))
  (Development|PrintString (Utilities|String|ToString(Text) (Utilities|Text|FormatText "user with id {id} name found {name}" UniqueNetID _value)))
  (return _value))