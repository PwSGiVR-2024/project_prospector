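; Deathmatch game mode that runs a timed match, tracks kills per player NetID and reloads via servertravel to Prototype_map when time expires.
; Tick counts down and, throttled by a delay gate, pushes the timer and scoreboard to every MainPlayerController.
; Respawns spawn a character at a random cached PlayerStart on authority, then possess it and create its HUD.
; Deaths broadcast a kill feed to all controllers and increment the killer's count.
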(event Custom|SendTime
  (if (not (Variables|Default|GetWaitingForSend))
    (Variables|Default|SetWaitingForSend true)
    (Utilities|FlowControl|Delay 0.5)
    (CallFunction|SendTimetoEveryone (Variables|Default|GetCurrentTime))
    (Variables|Default|SetWaitingForSend false)))

(event Custom|SendTimeToEveryone
  (params (timeInSeconds :type Float%20%28double-precision%29))
  (bind _outactors (Actor|GetAllActorsOfClass "/Game/Blueprints/MainPlayerController.MainPlayerController_C"))
  (for _array_element _outactors
    (Default|UpdateTimer _array_element timeInSeconds)
    (Default|UpdateCurrentScoreboard _array_element (Variables|Default|GetPlayerKills) (Variables|Default|GetUsers))))

(event EventPlayerDied
  (params (Who%20Died :type BP%20Third%20Person%20Character%20Object%20Reference) (Who%20Killed :type Actor%20Object%20Reference))
  (bind _playerkills (Variables|Default|GetPlayerKills))
  ;[1 1 1] PlayerDied
  (Utilities|FlowControl|Sequence
    (:then_0
      (|CallParentFunction Who%20Died Who%20Killed)
      (bind _asbp_third_person_character (Utilities|Casting|CastToBP_ThirdPersonCharacter Who%20Killed))
      (bind _asmain_player_controller (Utilities|Casting|CastToMainPlayerController (Pawn|GetController Who%20Died)))
      (bind _asmain_player_controller_2 (Utilities|Casting|CastToMainPlayerController (Pawn|GetController _asbp_third_person_character)))
      (bind _asbp_base_game_mode (Utilities|Casting|CastToBP_BaseGameMode (Game|GetGameMode)))
      (bind _name (Default|GetPlayerName _asbp_base_game_mode (Variables|/Game/Blueprints/MainPlayerController.MainPlayerController_C|GetNetID _asmain_player_controller)))
      (bind _name_2 (Default|GetPlayerName _asbp_base_game_mode (Variables|/Game/Blueprints/MainPlayerController.MainPlayerController_C|GetNetID _asmain_player_controller_2)))
      (bind _outactors (Actor|GetAllActorsOfClass "/Game/Blueprints/MainPlayerController.MainPlayerController_C"))
      (for _array_element _outactors
        (Default|ClientKillFeed _array_element (Utilities|Text|ToText(String) _name_2) (Variables|/Game/Blueprints/MainPlayerController.MainPlayerController_C|GetNetID _asmain_player_controller_2) (Utilities|Text|ToText(String) _name) (Variables|/Game/Blueprints/MainPlayerController.MainPlayerController_C|GetNetID _asmain_player_controller))))
    (:then_1
      (Utilities|Map|Add _playerkills (Variables|/Game/Blueprints/MainPlayerController.MainPlayerController_C|GetNetID _asmain_player_controller_2) (+ (.Value (Utilities|Map|Find _playerkills (Variables|/Game/Blueprints/MainPlayerController.MainPlayerController_C|GetNetID _asmain_player_controller_2))) 1))
      (Development|PrintString (Utilities|String|ToString(Text) (Utilities|Text|FormatText "{killer} kills: {kills}" (Utilities|Text|ToText(String) _name_2) (+ (.Value (Utilities|Map|Find _playerkills (Variables|/Game/Blueprints/MainPlayerController.MainPlayerController_C|GetNetID _asmain_player_controller_2))) 1))) true true "(R=0.000000,G=0.660000,B=1.000000,A=1.000000)" 1e+01))))

(event EventRespawnRequested
  (params (PlayerController :type Main%20Player%20Controller%20Object%20Reference) (Location :type Transform))
  ;[1 1 1] RespawnRequested
  (|CallParentFunction PlayerController Location)
  (Utilities|IsValid PlayerController
    (:Is%20Valid
      (Networking|SwitchHasAuthority
        (:Authority
          (bind _returnvalue (Game|SpawnActorfromClass "/Game/Blueprints/BP_ThirdPersonCharacter.BP_ThirdPersonCharacter_C" (Math|Conversions|ToTransform(Vector) (Transformation|GetActorLocation (.OutItem (Utilities|Array|Random (Variables|Default|GetPlayerStarts))))) "Undefined" "MultiplyWithRoot" 0 0))
          (Utilities|FlowControl|DelayUntilNextTick :!label _label)
          (Utilities|IsValid _returnvalue
            (:Is%20Valid
              (Pawn|Possess PlayerController _returnvalue)
              (Utilities|FlowControl|Delay 0.2)
              (Default|SpawnHud _returnvalue))
            (:Is%20Not%20Valid
              (goto _label))))))))

(event EventBeginPlay
  ;[1 1 1] BeginPlay
  (|CallParentFunction)
  (bind _outactors (Actor|GetAllActorsOfClass "/Script/Engine.PlayerStart"))
  (Variables|Default|SetPlayerStarts _outactors)
  (Variables|Default|SetCurrentTime (Variables|Default|GetMaxTime)))

(event EventTick
  (params (DeltaSeconds :type Float%20%28single-precision%29))
  ;[1 1 1] Tick
  (|CallParentFunction DeltaSeconds)
  (Utilities|FlowControl|Sequence
    (:then_0
      (Variables|Default|SetCurrentTime (- (Variables|Default|GetCurrentTime) DeltaSeconds))
      (CallFunction|SendTime))
    (:then_1
      (if (< (Variables|Default|GetCurrentTime) 0.0)
        (Networking|SwitchHasAuthority
          (:Authority
            (Development|ExecuteConsoleCommand "servertravel Prototype_map" 0)))))))

(event EventRegisterPlayer
  (params (Controller :type Controller%20Object%20Reference) (Name :type String%20%28by%20ref%29))
  (|CallParentFunction Controller Name)
  (bind _asmain_player_controller (Utilities|Casting|CastToMainPlayerController Controller))
  (Utilities|Map|Add (Variables|Default|GetPlayerKills) (Variables|/Game/Blueprints/MainPlayerController.MainPlayerController_C|GetNetID _asmain_player_controller) 0))

(fn ConstructionScript)