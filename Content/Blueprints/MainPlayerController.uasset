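; Player controller for a multiplayer deathmatch, linking each player to the game modes, the game instance's kill count and a local HUD.
; It forwards respawn, registration and death events to the game mode, and deaths also trigger RegisterKill on the killer's controller.
; HUD events update the timer and, on remotes only, the killfeed.
; ShowKillFeed looks up both names by NetID, but its ClientKillFeed call is disconnected.
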(event Custom|RespawnPawn
  (params (Location :type Transform))
  (bind _returnvalue (Game|GetGameMode))
  (Utilities|FlowControl|Delay 0.1)
  (Development|PrintString "main player controller respawn")
  (bind _asbp_base_game_mode (Utilities|Casting|CastToBP_BaseGameMode _returnvalue)
    (:then
      (Default|RespawnRequested _asbp_base_game_mode self Location))
    (:CastFailed
      (Development|PrintString (Utilities|GetDisplayName _returnvalue) true true "(R=1.000000,G=0.159370,B=0.000000,A=1.000000)" 5.0))))

(event Custom|RegisterItself
  (params (Name :type String))
  (bind _asbp_deathmatch_game_mode (Utilities|Casting|CastToBP_DeathmatchGameMode (Game|GetGameMode)))
  (Default|RegisterPlayer _asbp_deathmatch_game_mode self Name))

(event Custom|PlayerDiedInfo
  (params (Who%20Died :type BP%20Third%20Person%20Character%20Object%20Reference) (Who%20Killed :type Actor%20Object%20Reference))
  (bind _asbp_deathmatch_game_mode (Utilities|Casting|CastToBP_DeathmatchGameMode (Game|GetGameMode))
    (:then
      (Default|PlayerDied _asbp_deathmatch_game_mode Who%20Died Who%20Killed)
      (bind _asbp_third_person_character (Utilities|Casting|CastToBP_ThirdPersonCharacter Who%20Killed))
      (bind _asmain_player_controller (Utilities|Casting|CastToMainPlayerController (Pawn|GetController _asbp_third_person_character)))
      (CallFunction|RegisterKill _asmain_player_controller)
      (CallFunction|ShowKillFeed Who%20Died Who%20Killed))
    (:CastFailed
      (Development|PrintString "cast to deathmatch failder"))))

(event Custom|ShowKillFeed
  (params (Killed :type BP%20Third%20Person%20Character%20Object%20Reference) (Killer :type Actor%20Object%20Reference))
  (bind _asbp_third_person_character (Utilities|Casting|CastToBP_ThirdPersonCharacter Killer))
  (bind _asmain_player_controller (Utilities|Casting|CastToMainPlayerController (Pawn|GetController Killed)))
  (bind _asmain_player_controller_2 (Utilities|Casting|CastToMainPlayerController (Pawn|GetController _asbp_third_person_character)))
  (bind _asbp_base_game_mode (Utilities|Casting|CastToBP_BaseGameMode (Game|GetGameMode)))
  (bind _name (Default|GetPlayerName _asbp_base_game_mode (Variables|MainPlayerController_C|GetNetID _asmain_player_controller)))
  (bind _name_2 (Default|GetPlayerName _asbp_base_game_mode (Variables|MainPlayerController_C|GetNetID _asmain_player_controller_2))))

(event Custom|SpawnHud
  (if (Pawn|IsLocalController)
    (bind _returnvalue (UserInterface|CreateWidget "/Game/UI/HUD/ControllerHUD.ControllerHUD_C" 0 self))
    (bind _output_get (Variables|Default|SetControllerHUD _returnvalue))
    (UserInterface|Viewport|AddtoViewport _output_get -1)))

(event Custom|RegisterKill
  (bind _asmain_game_instance (Utilities|Casting|CastToMainGameInstance (Game|GetGameInstance)))
  (Default|AddKillforPlayer _asmain_game_instance (Variables|/Game/Blueprints/MainGameInstance.MainGameInstance_C|GetUsername _asmain_game_instance)))

(event Custom|ClientKillFeed
  (params (KillerName :type Text) (KillerNetID :type Integer) (VictimName :type Text) (VictimNetID :type Integer))
  (bind _controllerhud (Variables|Default|GetControllerHUD))
  (Networking|SwitchHasAuthority
    (:Remote
      (Utilities|IsValid _controllerhud
        (:Is%20Valid
          (Default|AddtoKillfeed (Variables|/Game/UI/HUD/ControllerHUD.ControllerHUD_C|GetKillfeedWidget _controllerhud) KillerName KillerNetID VictimName VictimNetID))))))

(event Custom|UpdateTimer
  (params (timeInSeconds :type Float%20%28double-precision%29))
  (CallFunction|UpdateTimerLocally timeInSeconds))

(event Custom|EventNetIDServer
  (params (NetID :type Integer))
  (Variables|Default|SetNetID NetID))

(event Custom|UpdateTimerLocally
  (params (timeInSeconds :type Float%20%28double-precision%29))
  (bind _controllerhud (Variables|Default|GetControllerHUD))
  (Utilities|IsValid _controllerhud
    (:Is%20Valid
      (Variables|/Game/UI/HUD/MatchTimer/TimerWidget.TimerWidget_C|SettimeInSeconds (Variables|/Game/UI/HUD/ControllerHUD.ControllerHUD_C|GetTimerWidget _controllerhud) timeInSeconds))))

(event EventBeginPlay)

(fn ConstructionScript)

(fn SetNetID
  (params (NetID :type Integer))
  (CallFunction|EventNetIDServer NetID)
  (return (Variables|Default|GetNetID)))