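; Inventory component that holds weapons in a fixed number of slots and tracks the active weapon index.
; Adding fills a requested empty slot or searches for one, falling back to the active slot; already-held weapons swap slots, while replacing an occupied requested slot is unimplemented.
; Swapping saves the current weapon's remaining ammo, then returns the selected weapon's data asset and ammo.
; A shared availability check backs the index validation macros, with failures printed on screen.
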(event Custom|InitializeWeaponArray
  (while (< (Utilities|Array|Length (Variables|Weapons|GetWeaponSlots)) (Variables|Weapons|GetMaxWeaponSlots))
    (Utilities|Array|Add (Variables|Weapons|GetWeaponSlots) 0)))

(event EventBeginPlay)

(event EventTick
  (params (DeltaSeconds :type Float%20%28single-precision%29)))

(fn AddWeapontoInventory
  (params (WeaponData :type Weapon%20Inventory%20Data%20Object%20Reference%20%28by%20ref%29) (ToInputIndex :type Boolean) (IndexSlot :type Integer))
  (bind _weaponslots (Variables|Weapons|GetWeaponSlots))
  ;[1 1 1] Check for duplicate weapon instance
  (if (not (Utilities|Array|ContainsItem (Variables|Weapons|GetWeaponSlots) WeaponData))
    (if ToInputIndex
      (Utilities|IsWeaponIndexViable IndexSlot
        (:true
          (Utilities|IsWeaponIndexEmpty IndexSlot
            (:true
              ;[1 1 1] Add Weapon to selected empty slot
              (Utilities|Array|SetArrayElem (Variables|Weapons|GetWeaponSlots) IndexSlot WeaponData))
            (:false
              (Utilities|PrintError "Attempted to replace weapon from another inventory while that functionality is not implemented yet, add")
              (return))))
        (:false
          (Utilities|PrintError "Attempted to add WeaponInventoryData to index out of bounds")
          (return)))
      (else
        ;[1 1 1] Search for empty weapon slot
        (bind _index (Utilities|FlowControl|ForLoopwithBreak 0 (Variables|Weapons|GetMaxWeaponSlots) :!label _label)
          (:LoopBody
            (Utilities|IsWeaponIndexEmpty _index
              (:true
                (LocalVariables|SetSearchSelectedIndex _index)
                (goto _label Break))))
          (:Completed
            (if (== (LocalVariables|GetSearchSelectedIndex) -1)
              ;[1 1 1] Add Weapon to active slot
              (Utilities|Array|SetArrayElem (Variables|Weapons|GetWeaponSlots) (Variables|Weapons|GetActiveWeaponIndex) WeaponData)
              (else
                ;[1 1 1] Add Weapon to empty slot
                (Utilities|Array|SetArrayElem (Variables|Weapons|GetWeaponSlots) (LocalVariables|GetSearchSelectedIndex) WeaponData)))))))
    (else
      ;[1 1 1] Weapon exists in current inventory - Swap index with input index
      (Utilities|IsWeaponIndexViable
        (:true
          (Utilities|Array|Swap _weaponslots (Utilities|Array|FindItem _weaponslots WeaponData) IndexSlot))
        (:false
          (Utilities|PrintError "Attempted to swap WeaponInventoryData index to index out of bounds")
          (return)))))
  (return))

(fn CheckWeaponIndexAvailability
  (params (Index :type Integer))
  (if (Math|Integer|InRange(Integer) Index 0 (Variables|Weapons|GetMaxWeaponSlots))
    (bind (_array_element _array_index) (Utilities|Array|ForEachLoopwithBreak (Variables|Weapons|GetWeaponSlots) :!label _label)
      (:LoopBody
        (if (and (Utilities|IsValid _array_element) (== _array_index Index))
          (LocalVariables|SetIndexAvailability false)
          (goto _label Break)))
      (:Completed
        (return (LocalVariables|GetIndexAvailability) true)))
    (else
      (Development|PrintText (Utilities|Text|FormatText "[WARNING] 
Source: {name} 
Function: CheckWeaponIndexAvailability 
Cause: Input index is out of available weapon slots range 
" (Utilities|GetObjectName self)) true true "(R=1.000000,G=0.935911,B=0.000000,A=1.000000)")
      (return false false))))

(fn GetWeaponfromSlot
  (params (WeaponIndex :type Integer))
  (bind (_isempty _isviable) (Weapons|CheckWeaponIndexAvailability WeaponIndex))
  (bind _weaponslots (Variables|Weapons|GetWeaponSlots))
  (bind _output (Utilities|Array|Get(acopy) _weaponslots WeaponIndex))
  (bind (_dataasset _ammoleft) (Default|FetchWeaponData _output))
  (if (and (not _isempty) _isviable)
    (return _dataasset _ammoleft true)
    (else
      (Utilities|PrintError "Cannot get Weapon Data: Weapon Slot is empty or out of bounds")
      (return 0 -1 false))))

(fn UpdateWeaponAmmo
  (params (WeaponIndex :type Integer) (AmmoLeft :type Integer))
  (bind (_isempty _isviable) (Weapons|CheckWeaponIndexAvailability WeaponIndex))
  (if (and (not _isempty) _isviable)
    (Default|SetAmmoLeft (Utilities|Array|Get(acopy) (Variables|Weapons|GetWeaponSlots) WeaponIndex) AmmoLeft)
    (else
      (Utilities|PrintError "Cannot modify Weapon Data: Weapon Slot is empty or out of bounds")))
  (return))

(fn UnequipCurrentWeapon
  (params (AmmoLeft :type Integer))
  (Weapons|UpdateWeaponAmmo (Variables|Weapons|GetActiveWeaponIndex) AmmoLeft)
  (return))

(fn SwapEquippedWeapon
  (params (AmmoLeftInCurrentWeapon :type Integer) (SelectedWeaponIndex :type Integer))
  (Weapons|UnequipCurrentWeapon AmmoLeftInCurrentWeapon)
  (bind (_dataasset _ammoleft _itemfound) (Weapons|EquipSelectedWeapon SelectedWeaponIndex))
  (return _dataasset _ammoleft _itemfound))

(fn EquipSelectedWeapon
  (params (WeaponIndex :type Integer))
  (bind (_dataasset _ammoleft _itemfound) (Weapons|GetWeaponfromSlot WeaponIndex))
  (if _itemfound
    (Variables|Weapons|SetActiveWeaponIndex WeaponIndex))
  (return _dataasset _ammoleft _itemfound))