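; BP_BaseClass is a base class that gives an actor health and a regenerating shield, initialised from BaseValues in the Construction Script.
; AnyDamage drains shield first, spills overflow into health, and restarts the affected regeneration delay.
; Tick counts down both delays independently, then regenerates each pool up to its maximum, printing values for debugging.
; The actor is destroyed when unshielded damage empties health; shield overflow skips that death check.
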(event Custom|HealthTimerEvent
  ;[1 1 1] Timer Events
  (Variables|Default|SetHealthTimer (Variables|/Game/DataAssets/Values/DAC_Base.DAC_Base_C|GetHealthTime (Variables|Default|GetBaseValues))))

(event Custom|RegenShield
  (params (Value :type Float%20%28double-precision%29))
  (bind _basevalues (Variables|Default|GetBaseValues))
  (bind _maxshield (Variables|/Game/DataAssets/Values/DAC_Base.DAC_Base_C|GetMaxShield _basevalues))
  ;[1 1 1] RegenShield
  (bind _output_get (Variables|Default|SetShield (+ (Variables|Default|GetShield) Value)))
  (if (> _output_get _maxshield)
    (Variables|Default|SetShield _maxshield)
    (else
      (Development|PrintString (Utilities|String|ToString(Float) _output_get) true true "(R=0.232226,G=0.000000,B=1.000000,A=1.000000)"))))

(event Custom|ShieldTimerEvent
  ;[1 1 1] Timer Events
  (Variables|Default|SetShieldTimer (Variables|/Game/DataAssets/Values/DAC_Base.DAC_Base_C|GetShieldTime (Variables|Default|GetBaseValues))))

(event Custom|RegenHealth
  (params (Value :type Float%20%28double-precision%29))
  (bind _basevalues (Variables|Default|GetBaseValues))
  (bind _maxhealth (Variables|/Game/DataAssets/Values/DAC_Base.DAC_Base_C|GetMaxHealth _basevalues))
  ;[1 1 1] RegenHealth
  (bind _output_get (Variables|Default|SetHealth (+ (Variables|Default|GetHealth) Value)))
  (if (> _output_get _maxhealth)
    (Variables|Default|SetHealth _maxhealth)
    (else
      (Development|PrintString (Utilities|String|ToString(Float) _output_get) true true "(R=0.211265,G=1.000000,B=0.000000,A=1.000000)"))))

(event Game|Damage|EventAnyDamage
  (params (Damage :type Float%20%28single-precision%29) (DamageType :type Damage%20Type%20Object%20Reference) (InstigatedBy :type Controller%20Object%20Reference) (DamageCauser :type Actor%20Object%20Reference))
  ;[1 1 1] Taking Damage
  (if (== (Variables|Default|GetShield) 0.0)
    (bind _output_get (Variables|Default|SetHealth (- (Variables|Default|GetHealth) Damage)))
    (Development|PrintString (Utilities|String|ToString(Float) _output_get) true true "(R=0.036666,G=0.229167,B=0.000000,A=1.000000)")
    (if (<= _output_get 0.0)
      (Actor|DestroyActor)
      (else
        (CallFunction|HealthTimerEvent :!label _label)))
    (else
      (bind _output_get_2 (Variables|Default|SetShield (- (Variables|Default|GetShield) Damage)))
      (Development|PrintString (Utilities|String|ToString(Float) _output_get_2) true true "(R=0.153592,G=0.000000,B=0.296875,A=1.000000)")
      (CallFunction|ShieldTimerEvent)
      (if (< (Variables|Default|GetShield) 0.0)
        (Variables|Default|SetHealth (+ (Variables|Default|GetHealth) (Variables|Default|GetShield)))
        (Variables|Default|SetShield 0.0)
        (goto _label)))))

(event EventTick
  (params (DeltaSeconds :type Float%20%28single-precision%29))
  (Variables|Default|SetDelta%20Seconds DeltaSeconds)
  (Utilities|FlowControl|Sequence
    (:then_0
      ;[1 1 1] Timers
      (if (> (Variables|Default|GetHealthTimer) 0.0)
        (Variables|Default|SetHealthTimer (- (Variables|Default|GetHealthTimer) (Variables|Default|GetDelta%20Seconds)))
        (else
          ;[1 1 1] Regeneration
          (CallFunction|RegenHealth (* (Variables|/Game/DataAssets/Values/DAC_Base.DAC_Base_C|GetHealthRegen (Variables|Default|GetBaseValues)) (Variables|Default|GetDelta%20Seconds))))))
    (:then_1
      (if (> (Variables|Default|GetShieldTimer) 0.0)
        (Variables|Default|SetShieldTimer (- (Variables|Default|GetShieldTimer) (Variables|Default|GetDelta%20Seconds)))
        (else
          (CallFunction|RegenShield (* (Variables|/Game/DataAssets/Values/DAC_Base.DAC_Base_C|GetShieldRegen (Variables|Default|GetBaseValues)) (Variables|Default|GetDelta%20Seconds))))))))

(fn ConstructionScript
  (bind _basevalues (Variables|Default|GetBaseValues))
  (Variables|Default|SetHealth (Variables|/Game/DataAssets/Values/DAC_Base.DAC_Base_C|GetMaxHealth _basevalues))
  (Variables|Default|SetShield (Variables|/Game/DataAssets/Values/DAC_Base.DAC_Base_C|GetMaxShield _basevalues))
  (Variables|Default|SetHealthTimer (Variables|/Game/DataAssets/Values/DAC_Base.DAC_Base_C|GetHealthTime _basevalues))
  (Variables|Default|SetShieldTimer (Variables|/Game/DataAssets/Values/DAC_Base.DAC_Base_C|GetShieldTime _basevalues)))