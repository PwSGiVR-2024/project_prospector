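; Blueprint interface that exposes player state queries, apparently for animation and other systems to read without casting to the player class.
; It declares getters for the left-hand socket transform, hand sway inputs from side movement and mouse axes, and the follow camera.
; Further getters report aiming, shooting with its elapsed time, crouching, and whether left-hand IK stops.
; The file holds only signatures with default returns, leaving the logic to implementing classes.
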(fn IFGetLeftHandSocketTransform
  (return ""))

(fn IFGetHandSwayFloats
  (return 0.0 0.0 0.0))

(fn IFGetAim
  (return false))

(fn IFGetShooting
  (return false 0.0))

(fn IFGetFollowCamera
  (return 0))

(fn IFGetCrouching
  (return false))

(fn IFStopLeftHandIK
  (return false))